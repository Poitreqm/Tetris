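; Line-clearing and score manager for a Tetris-style block game, creating the score widget on BeginPlay.
; CheckLines treats each BoxComponent overlapping exactly ten BP_SingleBlock actors as a full row, increasing DropAmount.
; If the box's Y is below CutOfLine, it stores the box's Z there, destroys the blocks and adds 0.1 points each.
; It then lowers every block above CutOfLine by DropAmount, which is never reset here.
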(event `self.ReceiveBeginPlay`
  (bind _returnvalue (`|CreateWidget` "/Game/Intefrace.Intefrace_C"))
  (bind _output_get (set `self.ScoreWidget` _returnvalue))
  (`UserWidget.AddToViewport` _output_get 0))

(event `AddPoints`
  (params (Points :type "Float (double-precision)"))
  (set `self.Score` (+ Points (`self.Score`)))
  (`/Game/Intefrace.UpdateScore` (`self.ScoreWidget`) (`self.Score`)))

(fn `CheckLines`
  (locals (overlappingActors :type "Array of Actor Object Reference") (dropAmount :type "Float (double-precision)") (cutOfLine :type "Float (double-precision)" :default 0.0) (Points :type "Float (double-precision)"))
  (for _array_element (`self.K2_GetComponentsByClass` "/Script/Engine.BoxComponent")
    (bind _output_get (set `local.overlappingActors` (`PrimitiveComponent.GetOverlappingActors` _array_element "/Game/BP_SingleBlock.BP_SingleBlock_C")))
    (if (== (`KismetArrayLibrary.Array_Length` _output_get) 10)
      (set `local.dropAmount` (+ (`local.dropAmount`) 50.0))
      (bind (_returnvalue_x _returnvalue_y _returnvalue_z) (`KismetMathLibrary.BreakVector` (`SceneComponent.K2_GetComponentLocation` _array_element)))
      (if (< _returnvalue_y (`local.cutOfLine`))
        (set `local.cutOfLine` _returnvalue_z)
        (for _array_element_2 (`local.overlappingActors`)
          ;[1 1 1] удаляется 10 объектво(количество клеточек в ряду) по этому что бы получить 1 очко ставим 0.1 за каждый удаленный блок
          (`self.K2_DestroyActor` _array_element_2)
          (`self.AddPoints` 0.1)))))
  (bind _outactors (`GameplayStatics.GetAllActorsOfClass` "/Game/BP_SingleBlock.BP_SingleBlock_C"))
  (for _array_element_3 _outactors
    (bind (_returnvalue_x_2 _returnvalue_y_2 _returnvalue_z_2) (`KismetMathLibrary.BreakVector` (`self.K2_GetActorLocation` _array_element_3)))
    (if (> _returnvalue_z_2 (`local.cutOfLine`))
      (`self.K2_SetActorLocation` _array_element_3 (`KismetMathLibrary.MakeVector` _returnvalue_x_2 _returnvalue_y_2 (- _returnvalue_z_2 (`local.dropAmount`))) false false))))

(fn `UserConstructionScript`)