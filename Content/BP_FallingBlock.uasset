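; Player-controlled falling Tetris-style piece that arranges four cubes into one of five random shapes on construction.
; A looping timer steps it down; downward traces detect landing, then it spawns BP_SingleBlock per cube, calls CheckLines, spawns its successor and destroys itself.
; Moves and rotations are applied, then reverted if box overlaps hit WorldStatic; squares skip rotation.
; Fast drop uses global time dilation, and random colour logic is unconnected.
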(event `self.ReceiveBeginPlay`
  (bind _returnvalue (`KismetSystemLibrary.K2_SetTimerDelegate` (delegate `DropBlock`) (`self.dropSpeed`) true))
  (set `self.blockDroppingTimer` _returnvalue))

(event `DropBlock`
  (bind _checklineactor (`self.checkLineActor`))
  (set `self.shouldDrop` true)
  (for _array_element (`SceneComponent.GetChildrenComponents` (`self.DefaultSceneRoot`) false)
    (bind _returnvalue (`SceneComponent.K2_GetComponentLocation` _array_element))
    (bind (_outhit _returnvalue_2) (`KismetSystemLibrary.LineTraceSingleForObjects` _returnvalue (- _returnvalue (0.0 0.0 50.0)) (`|MakeArray` "ObjectTypeQuery1" :!type "EObjectTypeQuery Enum")))
    (if _returnvalue_2
      (`/Engine/EditorBlueprintResources/StandardMacros.DoOnce` false
        (:`Completed`
          (set `self.shouldDrop` false)
          (`KismetSystemLibrary.K2_ClearAndInvalidateTimerHandle` (`self.blockDroppingTimer`))))))
  (if (`self.shouldDrop`)
    (`self.K2_AddActorWorldOffset` (0.0 0.0 -50.0))
    (else
      (for _array_element_2 (`SceneComponent.GetChildrenComponents` (`self.DefaultSceneRoot`) false)
        (`|SpawnActorFromClass` "/Game/BP_SingleBlock.BP_SingleBlock_C" (`KismetMathLibrary.MakeTransform` (`SceneComponent.K2_GetComponentLocation` _array_element_2)) "Undefined" "MultiplyWithRoot" null (struct) null))
      (`/Game/BP_CheckLine.CheckLines` _checklineactor)
      (`|SpawnActorFromClass` "BP_FallingBlock_C" (`KismetMathLibrary.MakeTransform` (25.0 0.0 1000.0)) "Undefined" "MultiplyWithRoot" null _checklineactor null)
      (`self.K2_DestroyActor`))))

(event `InputAction|MoveBlockRight`
  (params (Key :type "Key Structure"))
  (:`Pressed`
    (`self.MoveBlock` 50.0)))

(event `InputAction|MoveBlockLeft`
  (params (Key :type "Key Structure"))
  (:`Pressed`
    (`self.MoveBlock` -50.0)))

(event `InputAction|SpeedBlock`
  (params (Key :type "Key Structure"))
  (:`Pressed`
    (`GameplayStatics.SetGlobalTimeDilation` 5.0))
  (:`Released`
    (`GameplayStatics.SetGlobalTimeDilation` 1.0)))

(event `InputAction|RotateBlock`
  (params (Key :type "Key Structure"))
  (:`Pressed`
    (if (not (`self.isSquad`))
      (`self.K2_AddActorWorldRotation` (struct :`Pitch` 90.0))
      (for _array_element (`self.K2_GetComponentsByClass` "/Script/Engine.StaticMeshComponent")
        (bind (_outactors _returnvalue) (`KismetSystemLibrary.BoxOverlapActors` (`SceneComponent.K2_GetComponentLocation` _array_element) (15.0 15.0 15.0) (`|MakeArray` "ObjectTypeQuery1" :!type "EObjectTypeQuery Enum")))
        (if _returnvalue
          (`self.K2_AddActorWorldRotation` (struct :`Pitch` -90.0))
          (break))))))

(fn `MoveBlock`
  (params (Speed :type "Float (double-precision)"))
  (`self.K2_AddActorWorldOffset` (`KismetMathLibrary.MakeVector` Speed))
  (for _array_element (`self.K2_GetComponentsByClass` "/Script/Engine.StaticMeshComponent")
    (bind (_outactors _returnvalue) (`KismetSystemLibrary.BoxOverlapActors` (`SceneComponent.K2_GetComponentLocation` _array_element) (15.0 15.0 15.0) (`|MakeArray` "ObjectTypeQuery1" :!type "EObjectTypeQuery Enum")))
    (if _returnvalue
      (`self.K2_AddActorWorldOffset` (`KismetMathLibrary.MakeVector` (* Speed -1.0)))
      (break))))

(fn `UserConstructionScript`
  (switch `int` (`KismetMathLibrary.RandomIntegerInRange` 0 4)
    (:`0`
      ;[1 1 1] LINE BLOCK
      (`SceneComponent.K2_AddWorldOffset` (`self.Cube2`) (0.0 0.0 50.0) false false)
      (`SceneComponent.K2_AddWorldOffset` (`self.Cube3`) (0.0 0.0 100.0) false false)
      (`SceneComponent.K2_AddWorldOffset` (`self.Cube4`) (0.0 0.0 150.0) false false))
    (:`1`
      ;[1 1 1] L BLOCK
      (`SceneComponent.K2_AddWorldOffset` (`self.Cube2`) (50.0 0.0 0.0) false false)
      (`SceneComponent.K2_AddWorldOffset` (`self.Cube3`) (0.0 0.0 50.0) false false)
      (`SceneComponent.K2_AddWorldOffset` (`self.Cube4`) (0.0 0.0 100.0) false false))
    (:`2`
      ;[1 1 1] SQUAD BLOCK
      (`SceneComponent.K2_AddWorldOffset` (`self.Cube2`) (50.0 0.0 0.0) false false)
      (`SceneComponent.K2_AddWorldOffset` (`self.Cube3`) (0.0 0.0 50.0) false false)
      (`SceneComponent.K2_AddWorldOffset` (`self.Cube4`) (50.0 0.0 50.0) false false)
      ;[1 1 1] Если квадрат то не вертеть
      (set `self.isSquad` true))
    (:`3`
      ;[1 1 1] REVERSE LINE BLOCK
      (`SceneComponent.K2_AddWorldOffset` (`self.Cube2`) (50.0 0.0 0.0) false false)
      (`SceneComponent.K2_AddWorldOffset` (`self.Cube3`) (100.0 0.0 0.0) false false)
      (`SceneComponent.K2_AddWorldOffset` (`self.Cube4`) (150.0 0.0 0.0) false false))
    (:`4`
      ;[1 1 1] REVERSE L BLOCK
      (`SceneComponent.K2_AddWorldOffset` (`self.Cube2`) (0.0 0.0 -50.0) false false)
      (`SceneComponent.K2_AddWorldOffset` (`self.Cube3`) (-50.0 0.0 0.0) false false)
      (`SceneComponent.K2_AddWorldOffset` (`self.Cube4`) (-100.0 0.0 0.0) false false))))